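; BP_Projectile is a bullet for the VR tracking game that registers hits on player characters.
; On BeginPlay it launches its Sphere along the actor's right vector at the game state's BulletSpeed, with lifespan inversely scaled to speed for fixed range.
; Sphere overlaps ignore the character whose player state matches the stored NewVar, otherwise calling PlayerHit on the game mode and destroying the bullet.
; The game mode cast confines hits to the server.
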(event `self.ReceiveBeginPlay`
  ;[1 1 1] Init
  (bind _asvrtracking_game_state (cast `/CrewVRTracking/VRTrackingGameState` (`GameplayStatics.GetGameState`)))
  (bind _bulletspeed (`/CrewVRTracking/VRTrackingGameState.BulletSpeed` _asvrtracking_game_state))
  (`PrimitiveComponent.SetPhysicsLinearVelocity` (`self.Sphere`) (* (`KismetMathLibrary.GetRightVector` (`self.K2_GetActorRotation`)) _bulletspeed) false "None")
  (`self.SetLifeSpan` (/ 2000.0 _bulletspeed)))

(event `self.Sphere.OnComponentBeginOverlap`
  (params (OverlappedComponent :type "PrimitiveComponent Object Reference") (OtherActor :type "Actor Object Reference") (OtherComp :type "PrimitiveComponent Object Reference") (OtherBodyIndex :type Integer) (bFromSweep :type Boolean) (SweepResult :type "HitResult Structure (by ref)"))
  ;[1 1 1] Hit detection (Server Side)
  (bind _asvrtracking_game_mode (cast `/CrewVRTracking/VRTrackingGameMode` (`GameplayStatics.GetGameMode`)))
  (bind _asvrtracking_char (cast `/CrewVRTracking/Character/VRTrackingChar` OtherActor))
  (bind _asvrstate (cast `/CrewVRTracking/Character/VRState` (`Pawn.PlayerState` _asvrtracking_char)))
  (if (not (== _asvrstate (`self.NewVar`)))
    (`/CrewVRTracking/VRTrackingGameMode.PlayerHit` _asvrtracking_game_mode _asvrtracking_char)
    (`self.K2_DestroyActor`)))

(fn `UserConstructionScript`)